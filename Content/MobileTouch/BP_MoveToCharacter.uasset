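; Touch-controlled character for mobile, with standard axis bindings for yaw-relative movement and rate-based turn and look.
; Touch drags rotate the view: each move passes its location to UpdatePost, which adds the scaled delta from the last stored point as yaw and pitch.
; Pinch zoom is unfinished: it only prints a normalized change against the previous axis value, and the PinchZooming function is empty.
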(event Custom|UpdatePost
  (params (Update%20Post :type Vector%202D%20Structure))
  (bind _startlocation (Variables|Default|GetStartLocation))
  (bind _returnvalue (- Update%20Post _startlocation))
  (bind _returnvalue_2 (/ _returnvalue 5.0))
  (Pawn|Input|AddControllerYawInput (.x _returnvalue_2))
  (Pawn|Input|AddControllerPitchInput (.y _returnvalue_2)))

(event Input|AxisEvents|InputAxisPinchZoom
  (params (AxisValue :type Float%20%28single-precision%29))
  (if (not (== AxisValue (Variables|Default|GetPitchValue)))
    (Math|Float|CompareFloat AxisValue (Variables|Default|GetPitchValue)
      (:>
        (Development|PrintString (Utilities|String|ToString(Float) (- (Math|Float|Clamp(Float) (/ (Variables|Default|GetPitchValue) AxisValue)) 1.0))))
      (:<
        (Development|PrintString (Utilities|String|ToString(Float) (- 1.0 (Math|Float|Clamp(Float) (/ AxisValue (Variables|Default|GetPitchValue))))))))
    (Variables|Default|SetPitchValue AxisValue)))

(event Input|AxisEvents|InputAxisTurnRate
  (params (AxisValue :type Float%20%28single-precision%29))
  (Pawn|Input|AddControllerYawInput (* AxisValue (Variables|Default|GetBaseTurnRate) (Utilities|Time|GetWorldDeltaSeconds))))

(event Input|AxisEvents|InputAxisLookUpRate
  (params (AxisValue :type Float%20%28single-precision%29))
  (Pawn|Input|AddControllerPitchInput (* AxisValue (Variables|Default|GetBaseLookUpRate) (Utilities|Time|GetWorldDeltaSeconds))))

(event Input|AxisEvents|InputAxisMoveForward
  (params (AxisValue :type Float%20%28single-precision%29))
  (Pawn|Input|AddMovementInput (Math|Vector|GetForwardVector (Math|Rotator|MakeRotator 0.0 0.0 (.Yaw (Math|Rotator|BreakRotator (Pawn|GetControlRotation :!class /Script/Engine.Pawn))))) AxisValue false))

(event Input|AxisEvents|InputAxisMoveRight
  (params (AxisValue :type Float%20%28single-precision%29))
  (Pawn|Input|AddMovementInput (Math|Vector|GetRightVector (Math|Rotator|MakeRotator 0.0 0.0 (.Yaw (Math|Rotator|BreakRotator (Pawn|GetControlRotation :!class /Script/Engine.Pawn))))) AxisValue false))

(event Input|KeyboardEvents|GesturePinch
  (params (Key :type Key%20Structure :default "None")))

(event Input|TouchEvents|InputTouch
  (params (Location :type Vector) (FingerIndex :type ETouchIndex%20Enum))
  (bind (_x _y) (Math|Vector|BreakVector Location))
  (:Pressed
    (Variables|Default|SetStartLocation (Math|Vector2D|MakeVector2D _x _y) :!label _label))
  (:Released
    (goto _label))
  (:Moved
    (CallFunction|UpdatePost (Math|Vector2D|MakeVector2D _x _y))
    (goto _label)))

(fn ConstructionScript)

(fn PinchZooming)