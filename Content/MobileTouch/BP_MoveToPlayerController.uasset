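; Mobile touch player controller with logic to move the pawn to a tapped location, though its double-tap event chains are unconnected and never run.
; MoveToHitLocation skips hits closer than MinDistance to the pawn, then re-traces from the deprojected Touch1 screen position.
; It projects that trace point onto the navmesh, stores it in SaveLocation and calls SimpleMoveToLocation.
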(event EventBeginPlay)

(event EventTick
  (params (DeltaSeconds :type Float%20%28single-precision%29))
  ;[1 1 1] Move Character to Touch Position
)

(event Input|TouchEvents|InputTouch
  (params (Location :type Vector) (FingerIndex :type ETouchIndex%20Enum))
  ;[1 1 1] Move Character to Touch Position
)

(fn ConstructionScript)

(fn MovetoHitLocation
  (params (Hit :type Hit%20Result%20Structure))
  (bind _returnvalue (Game|GetPlayerController 0))
  (bind (_locationx _locationy) (Class|PlayerController|GetInputTouchState _returnvalue "Touch1"))
  (bind (_worldlocation _worlddirection) (Class|PlayerController|DeprojectScreenPositiontoWorld _returnvalue _locationx _locationy))
  ;[1 1 1] MoveToPosition
  (if (>= (Math|Vector|VectorLength (- (Transformation|GetActorLocation (Game|Player|GetPlayerPawn 0)) (.Location (Collision|BreakHitResult Hit)))) (Variables|Default|GetMin_Distance))
    (bind _outhit (Collision|LineTraceByChannel _worldlocation (+ _worldlocation (* _worlddirection 1e+03)) "TraceTypeQuery1" false 0 "None"))
    (Variables|Default|SetSaveLocation (.ProjectedLocation (AI|Navigation|ProjectPointtoNavigation (.Location (Collision|BreakHitResult _outhit)) 0 0 "0, 0, 0")))
    (AI|Navigation|SimpleMovetoLocation self (.ProjectedLocation (AI|Navigation|ProjectPointtoNavigation (.Location (Collision|BreakHitResult _outhit)) 0 0 "0, 0, 0")))))